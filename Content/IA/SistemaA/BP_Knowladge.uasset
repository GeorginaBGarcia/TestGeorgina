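; BP_Knowladge is an AI NPC character with a weapon, health and patrol support.
; On BeginPlay it spawns BP_Weapon on the mesh's Weapon socket.
; Damage lowers Life; a hit arriving at zero or below destroys NPC and weapon, while Tick updates the WB_HEALT bar and turns it toward the player.
; Helper functions set walk speed, return the next PatrolPath point while tracking its index, and expose the NPC itself.
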(event EventBeginPlay
  ;[1 1 1] Spawn Weapon
  (bind _returnvalue (Game|SpawnActorfromClass "/Game/BP_Weapon.BP_Weapon_C" (Transformation|GetSocketTransform (Variables|Character|GetMesh) "Weapon" "RTS_World") "Undefined" 0 0))
  (Transformation|AttachComponentToComponent _returnvalue (Variables|Character|GetMesh) "Weapon" "SnapToTarget" "SnapToTarget" "SnapToTarget" true))

(event Collision|EventActorBeginOverlap
  (params (OtherActor :type Actor%20Object%20Reference)))

(event EventTick
  (params (DeltaSeconds :type Float%20%28single-precision%29))
  ;[1 1 1] Widget
  (bind _aswb_healt (Utilities|Casting|CastToWB_HEALT (UserInterface|GetUserWidgetObject (Variables|Default|GetWidget))))
  (Progress|SetPercent (Variables|/Game/IA/SistemaB/WB_HEALT.WB_HEALT_C|GetProgressBar_0 _aswb_healt) (/ (Variables|Default|GetLife) 1e+02))
  (Transformation|SetWorldRotation (Variables|Default|GetWidget) (Math|Rotator|FindLookatRotation (Transformation|GetWorldLocation (Variables|Default|GetWidget)) (Transformation|GetActorLocation (Game|GetPlayerCharacter 0))) false false))

(event Game|Damage|EventAnyDamage
  (params (Damage :type Float%20%28single-precision%29) (DamageType :type Damage%20Type%20Object%20Reference) (InstigatedBy :type Controller%20Object%20Reference) (DamageCauser :type Actor%20Object%20Reference))
  ;[1 1 1] Damage
  (if (> (Variables|Default|GetLife) 0.0)
    (Variables|Default|SetLife (- (Variables|Default|GetLife) Damage))
    (else
      (Actor|DestroyActor)
      (Actor|DestroyActor (stale EventBeginPlay _returnvalue)))))

(fn ConstructionScript)

(fn UpdateWalkSpeed
  (params (New%20Walk%20Speed :type Float%20%28double-precision%29))
  (Variables|/Script/Engine.CharacterMovementComponent|SetMaxWalkSpeed (Variables|Character|GetCharacterMovement) New%20Walk%20Speed))

(fn GetNextPatrolPoint
  (bind _patrolpath (Variables|PATH|GetPatrolPath)
    (:then
      (bind (_newindex _targetlocation) (Default|GetPointLocation _patrolpath (+ (Variables|Default|GetCurrentSpinePosition) 1)))
      (Variables|Default|SetCurrentSpinePosition _newindex)
      (return _targetlocation))
    (:else
      (Development|PrintString "Patrol path is not valid check BP"))))

(fn GetNpc
  (return self))