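; AI enemy character that spawns with a weapon attached to its mesh socket and pursues the player.
; PawnSensing triggers a single AIMoveTo toward the player per sighting, which calls PlayAnimMontage on arrival within range.
; Damage lowers Life, and a hit received once Life is depleted destroys both character and weapon.
; Tick feeds Life into a health bar widget and rotates it to face the player.
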(event OnSeePawn(PawnSensing)
  (params (Pawn :type Pawn%20Object%20Reference))
  ;[1 1 1] IA MOVEMENT
  (Variables|Default|SetIsSeePlayer? true)
  (CallFunction|FollowPlayer))

(event Custom|Follow%20Player
  ;[1 1 1] IA MOVEMENT
  (if (Variables|Default|GetIsSeePlayer?)
    (AI|AIMoveTo self "0, 0, 0" (Game|GetPlayerCharacter 0) 5e+02 false
      (:OnSuccess
        (Animation|PlayAnimMontage 0 1.0 "None")))))

(event EventBeginPlay
  ;[1 1 1] SpawnWeapon
  (bind _returnvalue (Game|SpawnActorfromClass "/Game/BP_Weapon.BP_Weapon_C" (Transformation|GetSocketTransform (Variables|Character|GetMesh) "WeaponSocket_0" "RTS_World") "Undefined" 0 0))
  (Transformation|AttachComponentToComponent _returnvalue (Variables|Character|GetMesh) "WeaponSocket_0" "SnapToTarget" "SnapToTarget" "SnapToTarget" true))

(event Collision|EventActorBeginOverlap
  (params (OtherActor :type Actor%20Object%20Reference)))

(event EventTick
  (params (DeltaSeconds :type Float%20%28single-precision%29))
  ;[1 1 1] Widget
  (bind _aswb_healt (Utilities|Casting|CastToWB_HEALT (UserInterface|GetUserWidgetObject (Variables|Default|GetWidget))))
  (Progress|SetPercent (Variables|/Game/IA/SistemaB/WB_HEALT.WB_HEALT_C|GetProgressBar_0 _aswb_healt) (/ (Variables|Default|GetLife) 1e+02))
  (Transformation|SetWorldRotation (Variables|Default|GetWidget) (Math|Rotator|FindLookatRotation (Transformation|GetWorldLocation (Variables|Default|GetWidget)) (Transformation|GetActorLocation (Game|GetPlayerCharacter 0))) false false))

(event Game|Damage|EventAnyDamage
  (params (Damage :type Float%20%28single-precision%29) (DamageType :type Damage%20Type%20Object%20Reference) (InstigatedBy :type Controller%20Object%20Reference) (DamageCauser :type Actor%20Object%20Reference))
  ;[1 1 1] Damage
  (if (> (Variables|Default|GetLife) 0.0)
    (Variables|Default|SetLife (- (Variables|Default|GetLife) Damage))
    (else
      (Actor|DestroyActor)
      (Actor|DestroyActor (stale EventBeginPlay _returnvalue)))))

(fn ConstructionScript)